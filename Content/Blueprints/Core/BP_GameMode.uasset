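; Game mode that acts as the UI screen manager and handles menu actions and streamed level loading.
; MainSetup retries until it gets BP_GameInstance, then creates a hidden widget per ScreensArray entry.
; ShowScreen and HideScreens fade widgets, with ShowScreen also setting input mode and cursor; Credits and Pause Menu widgets are never created here.
; LoadLevel fades in the loading screen, streams the level when that animation finishes, then fades out after a fixed delay.
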(event `self.ReceiveBeginPlay`
  (`self.MainSetup`))

(event `MainSetup`
  (bind _asbp_game_instance (cast `/Game/Blueprints/Core/BP_GameInstance` (`GameplayStatics.GetGameInstance`))
    (:`then`
      (bind _output_get (set `self.GameInstance_Ref` _asbp_game_instance))
      (`/Engine/EditorBlueprintResources/StandardMacros.IsValid` _output_get
        (:`Is Valid`
          (`KismetSystemLibrary.Delay` 0.2)
          (`self.InitializeUI`))
        (:`Is Not Valid`
          (`KismetSystemLibrary.K2_SetTimerDelegate` (delegate `MainSetup`) 0.2 :!label _label))))
    (:`CastFailed`
      (goto _label))))

(event `InitializeUI`
  (for _array_element (`/Game/Blueprints/Core/BP_GameInstance.ScreensArray` (`self.GameInstance_Ref`))
    (`KismetSystemLibrary.PrintString` (`KismetStringLibrary.Concat_StrStr` "SCREEN SETUP: " (`|GetEnumeratorNameAsString` _array_element)))
    (switch `/Game/Blueprints/Data/ENUM_Screens` _array_element
      (:`NewEnumerator0`
        (`self.InitializeUI_LoadingGame`))
      (:`NewEnumerator1`
        (`self.InitializeUI_LoadingLevel`))
      (:`NewEnumerator2`
        (`self.InitializeUI_MainMenu`))
      (:`NewEnumerator3`
        (`self.InitializeUI_Options`))
      (:`NewEnumerator6`
        (`self.InitializeUI_Gameplay`)))))

(event `FadeInLoadingGame`
  (`/Game/UI/UI_LoadingGame.FadeIn` (`self.UI_LoadingGame_Ref`)))

(event `FadeInLoadingLevel`
  (`/Game/UI/UI_LoadingLevel.FadeIn` (`self.UI_LoadingLevel_Ref`)))

(event `FadeOutLoadingGame`
  (`/Game/UI/UI_LoadingGame.FadeOut` (`self.UI_LoadingGame_Ref`)))

(event `FadeOutLoadingLevel`
  (`/Game/UI/UI_LoadingLevel.FadeOut` (`self.UI_LoadingLevel_Ref`)))

(event `LoadLevel`
  (params (LevelName :type "/Game/Blueprints/Data/ENUM_Maps Enum" :default "NewEnumerator0"))
  (`self.FadeInLoadingLevel`)
  (add `/Game/UI/UI_Animation.FadeAnimationFinished` (`self.UI_LoadingLevel_Ref`) (delegate `LoadingProcess`))
  (`self.HideScreens`))

(event `LoadingProcess`
  (`GameplayStatics.LoadStreamLevel` (`KismetStringLibrary.Conv_StringToName` (`|GetEnumeratorNameAsString` (stale `LoadLevel` LevelName))) true)
  (remove `/Game/UI/UI_Animation.FadeAnimationFinished` (`self.UI_LoadingLevel_Ref`) (delegate `LoadingProcess`))
  (`KismetSystemLibrary.Delay` 1.0)
  (`self.FadeOutLoadingLevel`))

(event `MainMenu_Start`
  (`self.LoadLevel` "NewEnumerator4"))

(event `MainMenu_Credits`
  (`self.ShowScreen` "NewEnumerator4"))

(event `MainMenu_Options`
  (`self.ShowScreen` "NewEnumerator3"))

(event `MainMenu_Quit`
  (`KismetSystemLibrary.QuitGame` null "Quit"))

(fn `HideScreen`
  (params (ScreenName :type "/Game/Blueprints/Data/ENUM_Screens Enum" :default "NewEnumerator0"))
  (bind _ui_mainmenu_ref (`self.UI_MainMenu_Ref`))
  (bind _ui_options_ref (`self.UI_Options_Ref`))
  (bind _ui_gameplay_ref (`self.UI_Gameplay_Ref`))
  (switch `/Game/Blueprints/Data/ENUM_Screens` ScreenName
    (:`NewEnumerator2`
      (if (`Widget.IsVisible` _ui_mainmenu_ref)
        (`/Game/UI/UI_Animation.FadeOut` _ui_mainmenu_ref)))
    (:`NewEnumerator3`
      (if (`Widget.IsVisible` _ui_options_ref)
        (`/Game/UI/UI_Animation.FadeOut` _ui_options_ref)))
    (:`NewEnumerator6`
      (if (`Widget.IsVisible` _ui_gameplay_ref)
        (`/Game/UI/UI_Animation.FadeOut` _ui_gameplay_ref)))))

(fn `HideScreens`
  (locals (CurrentWidget :type "Widget Object Reference"))
  (for _array_element (`/Game/Blueprints/Core/BP_GameInstance.ScreensArray` (`self.GameInstance_Ref`))
    (`self.HideScreen` _array_element)))

(fn `InitializeUI_Gameplay`
  (bind _returnvalue (`|CreateWidget` "/Game/UI/UI_Gameplay.UI_Gameplay_C"))
  (bind _output_get (set `self.UI_Gameplay_Ref` _returnvalue))
  (`Widget.SetVisibility` _output_get "Hidden")
  (`UserWidget.AddToViewport` _output_get 0)
  (`KismetArrayLibrary.Array_Add` (`self.UI_Widgets`) _output_get))

(fn `InitializeUI_LoadingGame`
  (bind _returnvalue (`|CreateWidget` "/Game/UI/UI_LoadingGame.UI_LoadingGame_C"))
  (bind _output_get (set `self.UI_LoadingGame_Ref` _returnvalue))
  (`Widget.SetVisibility` _output_get "Hidden")
  (`UserWidget.AddToViewport` _output_get 0))

(fn `InitializeUI_LoadingLevel`
  (bind _returnvalue (`|CreateWidget` "/Game/UI/UI_LoadingLevel.UI_LoadingLevel_C"))
  (bind _output_get (set `self.UI_LoadingLevel_Ref` _returnvalue))
  (`Widget.SetVisibility` _output_get "Hidden")
  (`UserWidget.AddToViewport` _output_get 0))

(fn `InitializeUI_MainMenu`
  (bind _returnvalue (`|CreateWidget` "/Game/UI/UI_MainMenu.UI_MainMenu_C"))
  (bind _output_get (set `self.UI_MainMenu_Ref` _returnvalue))
  (`Widget.SetVisibility` _output_get "Hidden")
  (`UserWidget.AddToViewport` _output_get 0)
  (`KismetArrayLibrary.Array_Add` (`self.UI_Widgets`) _output_get))

(fn `InitializeUI_Options`
  (bind _returnvalue (`|CreateWidget` "/Game/UI/UI_Options.UI_Options_C"))
  (bind _output_get (set `self.UI_Options_Ref` _returnvalue))
  (`Widget.SetVisibility` _output_get "Hidden")
  (`UserWidget.AddToViewport` _output_get 0)
  (`KismetArrayLibrary.Array_Add` (`self.UI_Widgets`) _output_get))

(fn `ShowScreen`
  (params (Screen :type "/Game/Blueprints/Data/ENUM_Screens Enum" :default "NewEnumerator0"))
  (bind _returnvalue (`GameplayStatics.GetPlayerController` 0))
  (bind _ui_options_ref (`self.UI_Options_Ref`))
  (bind _ui_mainmenu_ref (`self.UI_MainMenu_Ref`))
  (bind _ui_credits_ref (`self.UI_Credits_Ref`))
  (bind _ui_pausemenu_ref (`self.UI_PauseMenu_Ref`))
  (switch `/Game/Blueprints/Data/ENUM_Screens` Screen
    (:`NewEnumerator2`
      (`self.HideScreens`)
      (`/Game/UI/UI_Animation.FadeIn` _ui_mainmenu_ref)
      (`WidgetBlueprintLibrary.SetInputMode_GameAndUIEx` (`GameplayStatics.GetPlayerController` 0) _ui_mainmenu_ref "DoNotLock" false)
      (set `PlayerController.bShowMouseCursor` true (`GameplayStatics.GetPlayerController` 0) :!label _label))
    (:`NewEnumerator3`
      (`/Game/UI/UI_Animation.FadeIn` _ui_options_ref)
      (`WidgetBlueprintLibrary.SetInputMode_GameAndUIEx` (`GameplayStatics.GetPlayerController` 0) _ui_options_ref "DoNotLock" false)
      (goto _label))
    (:`NewEnumerator4`
      (`self.HideScreens`)
      (`/Game/UI/UI_Animation.FadeIn` _ui_credits_ref)
      (`WidgetBlueprintLibrary.SetInputMode_GameAndUIEx` (`GameplayStatics.GetPlayerController` 0) _ui_credits_ref "DoNotLock" false)
      (goto _label))
    (:`NewEnumerator5`
      (`/Game/UI/UI_Animation.FadeIn` _ui_pausemenu_ref)
      (`WidgetBlueprintLibrary.SetInputMode_GameAndUIEx` (`GameplayStatics.GetPlayerController` 0) _ui_pausemenu_ref "DoNotLock" false)
      (goto _label))
    (:`NewEnumerator6`
      (`self.HideScreens`)
      (`/Game/UI/UI_Animation.FadeIn` (`self.UI_Gameplay_Ref`))
      (`WidgetBlueprintLibrary.SetInputMode_GameOnly` _returnvalue)
      (set `PlayerController.bShowMouseCursor` false _returnvalue))))

(fn `UserConstructionScript`)